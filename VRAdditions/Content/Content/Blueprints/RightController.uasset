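; RightController is an actor Blueprint for the right-hand VR motion controller that logs its tracking data for diagnostics.
; It enables input for player 0 on BeginPlay.
; Each Tick, while the MotionController component is tracked, it reads right-hand controller data and logs device name, hand index, grip position and rotation, and aim position.
; The log text is labelled "Left Hand" despite querying the right hand.
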(event `self.ReceiveBeginPlay`
  (`self.EnableInput` (`GameplayStatics.GetPlayerController` 0)))

(event `self.ReceiveTick`
  (params (DeltaSeconds :type "Float (single-precision)"))
  (bind _motioncontroller (`self.MotionController`))
  (if (`MotionControllerComponent.IsTracked` _motioncontroller)
    (bind _motioncontrollerdata (`HeadMountedDisplayFunctionLibrary.GetMotionControllerData` _motioncontroller "Right"))
    (bind (_bvalid _devicename _applicationinstanceid _devicevisualtype _handindex _trackingstatus _gripposition _griprotation _aimposition) (break `XRMotionControllerData` _motioncontrollerdata))
    (bind (_x _y _z _w) (`KismetMathLibrary.BreakQuat` _griprotation))
    (`BlueprintLoggingLibrary.LogDisplay` (`KismetStringLibrary.Concat_StrStr` "Left Hand Data Name: " (`KismetStringLibrary.Conv_NameToString` _devicename) "Hand Index : " (`|GetEnumeratorNameAsString` _handindex) "Grips : " (`KismetStringLibrary.Conv_VectorToString` _gripposition) (`KismetStringLibrary.Concat_StrStr` (`KismetStringLibrary.Conv_DoubleToString` _x) (`KismetStringLibrary.Conv_DoubleToString` _y) (`KismetStringLibrary.Conv_DoubleToString` _z) (`KismetStringLibrary.Conv_DoubleToString` _w)) "Aim : " (`KismetStringLibrary.Conv_VectorToString` _aimposition)))))

(fn `UserConstructionScript`)